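; BP_SwingWood is a swinging trap that kills the top-down character on contact.
; BeginPlay stores the starting rotation and a target pitched 90 degrees down from it.
; Tick runs through a Delay that periodically restarts the SwingBlade timeline, whose track lerps the actor's rotation between the two.
; A box collision overlap casts to BP_TopDownCharacter and calls Death.
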(event OnComponentBeginOverlap(BoxCollision)
  (params (OverlappedComponent :type Primitive%20Component%20Object%20Reference) (OtherActor :type Actor%20Object%20Reference) (OtherComp :type Primitive%20Component%20Object%20Reference) (OtherBodyIndex :type Integer) (bFromSweep :type Boolean) (SweepResult :type Hit%20Result%20Structure%20%28by%20ref%29))
  (bind _asbp_top_down_character (Utilities|Casting|CastToBP_TopDownCharacter OtherActor))
  (Default|Death _asbp_top_down_character))

(event EventBeginPlay
  (bind _returnvalue (Transformation|GetActorRotation))
  (bind (_roll _pitch _yaw) (Math|Rotator|BreakRotator _returnvalue))
  (Variables|Default|SetCurrentPosition _returnvalue)
  (Variables|Default|SetSwingTo (Math|Rotator|MakeRotator _roll (+ _pitch -9e+01) _yaw)))

(event EventTick
  (params (DeltaSeconds :type Float%20%28single-precision%29))
  (Utilities|FlowControl|Delay 4.0)
  (bind _swingblade_track (Timeline|SwingBlade PlayFromStart)
    (:Update
      (Transformation|SetActorRotation (Math|Rotator|Lerp(Rotator) (Variables|Default|GetCurrentPosition) (Variables|Default|GetSwingTo) _swingblade_track)))))

(fn ConstructionScript)